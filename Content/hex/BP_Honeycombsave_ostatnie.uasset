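; BP_Honeycombsave_ostatnie is a grid builder that lays out child actors, apparently as a honeycomb, from Rows and Cols counts.
; Its construction script destroys existing child actor components, then adds one per cell in a nested loop.
; Row parity alters the X spacing and column parity the Y spacing, each multiplied by the cell index rather than added as a fixed stagger.
; The event graph holds only disabled stubs.
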(fn `UserConstructionScript`
  (for _array_element (`self.K2_GetComponentsByClass` "/Script/Engine.ChildActorComponent")
    (`ActorComponent.K2_DestroyComponent` _array_element))
  (for _index (range (`self.Rows`))
    (for _index_2 (range (`self.Cols`))
      (`AddComponent|NODE_AddChildActorComponent-1` :`RelativeTransform` (`KismetMathLibrary.MakeTransform` (`KismetMathLibrary.MakeVector` (* (`KismetMathLibrary.Conv_IntToDouble` _index_2) (+ 86.7 (`KismetMathLibrary.SelectFloat` 0.0 86.5 (== (mod _index 2) 1)))) (* (`KismetMathLibrary.Conv_IntToDouble` _index) (+ 150.0 (`KismetMathLibrary.SelectFloat` 0.0 150.0 (== (mod _index_2 2) 1))))))))))